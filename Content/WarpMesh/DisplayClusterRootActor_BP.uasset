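; nDisplay root actor for virtual production, driving in-camera tracking and remote stage control over OSC.
; Each tick copies offset-corrected tracker pose to CineCam and BMCapture, sends it to a hardcoded OSC address, and applies stage offsets to the cluster root.
; An OSC server, restarted when inactive, takes TouchOSC/Companion commands for stage placement, wall rotation nudges, frustum, chromakey, lens, level swaps and multi-user connection.
; The J key separately joins an available online session.
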(event `self.ReceiveBeginPlay`
  (bind _returnvalue (`GameplayStatics.GetActorOfClass` "/nDisplay/Blueprints/ReprojectionCamera/BP_IncameraSettings.BP_IncameraSettings_C"))
  (`/Engine/EditorBlueprintResources/StandardMacros.IsValid` _returnvalue
    (:`Is Valid`
      (set `self.CineCam` (`/nDisplay/Blueprints/ReprojectionCamera/BP_IncameraSettings.ReprojectedCineCamera` _returnvalue))
      (`KismetSystemLibrary.PrintString` "Cam-Established")
      (set `self.OffsetOrigin` (0.0 0.0 0.0))
      (`self.StartOSC`))))

(event `self.ReceiveTick`
  (params (DeltaSeconds :type "Float (single-precision)"))
  (bind _cinecam (`self.CineCam`))
  (bind _deviceid (`self.DeviceID`))
  (bind _bmcapture (`self.BMCapture`))
  (bind _asdisplay_cluster_blueprint_apiimpl (cast `DisplayClusterBlueprintAPIImpl` (`DisplayClusterBlueprintLib.GetAPI`)))
  (bind _location (`DisplayClusterBlueprintAPIImpl.GetTrackerLocation` _asdisplay_cluster_blueprint_apiimpl _deviceid 0))
  (bind _rotation (`DisplayClusterBlueprintAPIImpl.GetTrackerQuat` _asdisplay_cluster_blueprint_apiimpl _deviceid 0))
  (bind _returnvalue (- _location (`self.OffsetOrigin`)))
  (`self.K2_SetActorRelativeLocation` _cinecam _returnvalue false false)
  (bind _returnvalue_2 (`KismetMathLibrary.Quat_Rotator` _rotation))
  (`self.K2_SetActorRelativeRotation` _cinecam _returnvalue_2 false false)
  (`self.K2_SetActorRelativeLocation` _bmcapture _returnvalue false false)
  (`self.K2_SetActorRelativeRotation` _bmcapture _returnvalue_2 false false)
  (bind _returnvalue_3 (`OSCManager.CreateOSCClient` "192.168.1.201" 8000))
  (bind _returnvalue_4 (`OSCManager.ConvertStringToOSCAddress` "/unrealvp/tracksend/location"))
  (bind _returnvalue_5 (`OSCManager.SetOSCMessageAddress` (make `OSCMessage`) _returnvalue_4))
  (bind _returnvalue_6 (`OSCManager.AddFloat` _returnvalue_5 (.x _returnvalue)))
  (bind _returnvalue_7 (`OSCManager.AddFloat` _returnvalue_6 (.y _returnvalue)))
  (bind _returnvalue_8 (`OSCManager.AddFloat` _returnvalue_7 (.z _returnvalue)))
  (`OSCClient.SendOSCMessage` _returnvalue_3 _returnvalue_8)
  (bind _returnvalue_9 (`OSCManager.ConvertStringToOSCAddress` "/unrealvp/tracksend/rotation"))
  (bind _returnvalue_10 (`OSCManager.SetOSCMessageAddress` (make `OSCMessage`) _returnvalue_9))
  (bind (_x _y _z) (`KismetMathLibrary.BreakQuat` _rotation))
  (bind _returnvalue_11 (`OSCManager.AddFloat` _returnvalue_10 _x))
  (bind _returnvalue_12 (`OSCManager.AddFloat` _returnvalue_11 _y))
  (bind _returnvalue_13 (`OSCManager.AddFloat` _returnvalue_12 _z))
  (`OSCClient.SendOSCMessage` _returnvalue_3 _returnvalue_13)
  (`self.Stage Track`)
  (`self.Check OSC Server`))

(event `ChangeViveOffset`
  (params (OriginOffset :type "Vector Structure"))
  (set `self.OffsetOrigin` OriginOffset))

(event `StartOSC`
  ;[1 1 1] Setup the OSC Server
  (bind _returnvalue (`OSCManager.CreateOSCServer` (`self.OSC IP Address`) (`self.OSC Port`) false true)) ; Setup the OSC Server with the IP/Port \nSpecified in the editor
  (bind _output_get (set `self.OSC Server` _returnvalue)) ; Set the OSC Server so we can \nreference it later
  (bind _returnvalue_2 (`OSCManager.ConvertStringToOSCAddress` "/UnrealVP/time")) ; Listen for a specific URL - This one doesn't\nreally do anything, TouchOSC is supposed to\nsend this URL if you're using the clock but it \ndoesn't seem to, nor does /ping work...
  (`OSCServer.BindEventToOnOSCAddressPatternMatchesPath` _output_get _returnvalue_2 (delegate `Reset OSC Ping Seconds`)) ; Call an event if the OSC address pattern is matched and/or \ncontinue to the next step to the right
  (bind _returnvalue_3 (`OSCManager.ConvertStringToOSCAddress` "/UnrealVP/accxyz")) ; This string is supposed to get accelerometer \ndata from the iPad. It doesn't work for whatever\nreason.. Would be real useful if it did!
  (`OSCServer.BindEventToOnOSCAddressPatternMatchesPath` _output_get _returnvalue_3 (delegate `Test ACCXYZ`))
  (bind _returnvalue_4 (`OSCManager.ConvertStringToOSCAddress` "/unreal/messages")) ; Map this to a toggle button to turn warning\nmessages ON or OFF
  (`OSCServer.BindEventToOnOSCAddressPatternMatchesPath` _output_get _returnvalue_4 (delegate `Message Toggle`))
  (bind _returnvalue_5 (`OSCManager.ConvertStringToOSCAddress` "/unreal/ndisplay/fov/offset")) ; This changes the FOV offset paramter up/down from a\nslider, making the square that the camera is looking at\nbigger or smaller. It's using an increment rather than setting\nvalues directly as I got better results doing it this way
  (`OSCServer.BindEventToOnOSCAddressPatternMatchesPath` _output_get _returnvalue_5 (delegate `Change FOV Offset`))
  (bind _returnvalue_6 (`OSCManager.ConvertStringToOSCAddress` "/unreal/ndisplay/stage/location/YZ")) ; This maps to a 2 axis fader in touch OSC to adjust the \nstage location. Weirdly it snaps back to where it was after\nyou stop sending the OSC message...
  (`OSCServer.BindEventToOnOSCAddressPatternMatchesPath` _output_get _returnvalue_6 (delegate `Update Stage Location YZ`))
  (bind _returnvalue_7 (`OSCManager.ConvertStringToOSCAddress` "/unreal/ndisplay/stage/location/X")) ; A single fader to do the X location offset
  (`OSCServer.BindEventToOnOSCAddressPatternMatchesPath` _output_get _returnvalue_7 (delegate `Update Location X`))
  (bind _returnvalue_8 (`OSCManager.ConvertStringToOSCAddress` "/unreal/ndisplay/stage/rotation/YZ")) ; Set the stage rotation offset using a 2 axis fader
  (`OSCServer.BindEventToOnOSCAddressPatternMatchesPath` _output_get _returnvalue_8 (delegate `Update Stage Rotation YZ`))
  (set `self.Last OSC Message` 0) ; These variable sets are just littered about\nto say that the OSC server is still running\ndon't pay them too much mind..
  (bind _returnvalue_9 (`OSCManager.ConvertStringToOSCAddress` "/unreal/ndisplay/stage/rotation/X")) ; Get the stage rotation X
  (`OSCServer.BindEventToOnOSCAddressPatternMatchesPath` _output_get _returnvalue_9 (delegate `Update Stage Rotation X`))
  (bind _returnvalue_10 (`OSCManager.ConvertStringToOSCAddress` "/unreal/ndisplay/chromakey/capture")) ; This is a button to turn the chromakey box on/OFF\nIt hasn't been implemented yet in the project
  (`OSCServer.BindEventToOnOSCAddressPatternMatchesPath` _output_get _returnvalue_10 (delegate `Enable Chromakey Capture`))
  (bind _returnvalue_11 (`OSCManager.ConvertStringToOSCAddress` "/unreal/ndisplay/chromakey/blur")) ; This should toggle a blur on the chromakey
  (`OSCServer.BindEventToOnOSCAddressPatternMatchesPath` _output_get _returnvalue_11 (delegate `Enable Chromakey Blur`))
  (bind _returnvalue_12 (`OSCManager.ConvertStringToOSCAddress` "/unreal/ndisplay/stage/nudge/rotz")) ; This is meant to nudge the stage rotationZ
  (`OSCServer.BindEventToOnOSCAddressPatternMatchesPath` _output_get _returnvalue_12 (delegate `Nudge Stage RotZ`))
  (bind _returnvalue_13 (`OSCManager.ConvertStringToOSCAddress` "/unreal/ndisplay/stage/nudge/roty")) ; This is meant to nudge the stage rotation Y
  (`OSCServer.BindEventToOnOSCAddressPatternMatchesPath` _output_get _returnvalue_13 (delegate `Nudge Stage RotY`))
  (bind _returnvalue_14 (`OSCManager.ConvertStringToOSCAddress` "/unreal/ndisplay/stage/nudge/rotx")) ; This is meant to nudge the X rotation
  (`OSCServer.BindEventToOnOSCAddressPatternMatchesPath` _output_get _returnvalue_14 (delegate `Nudge Stage RotX`))
  (bind _returnvalue_15 (`OSCManager.ConvertStringToOSCAddress` "/unreal/hostmultiplayer")) ; Not implemented yet
  (`OSCServer.BindEventToOnOSCAddressPatternMatchesPath` _output_get _returnvalue_15 (delegate `StartOnlineSesh`))
  (bind _returnvalue_16 (`OSCManager.ConvertStringToOSCAddress` "/unreal/ndisplay/frustum/feather")) ; This makes the edge around the camera frustrum \nclearer or blurrier
  (`OSCServer.BindEventToOnOSCAddressPatternMatchesPath` _output_get _returnvalue_16 (delegate `Adjust Frustum Feather`))
  (bind _returnvalue_17 (`OSCManager.ConvertStringToOSCAddress` "/unreal/camera//dof/focaldistance")) ; Change the DOF Focal Distance
  (`OSCServer.BindEventToOnOSCAddressPatternMatchesPath` _output_get _returnvalue_17 (delegate `Set Camera DOF Focal Distance`))
  (bind _returnvalue_18 (`OSCManager.ConvertStringToOSCAddress` "/unreal/camera/dof/blur/radius")) ; Change the DOF Blur Radius
  (`OSCServer.BindEventToOnOSCAddressPatternMatchesPath` _output_get _returnvalue_18 (delegate `Set Camera DOF Blur Radius`))
  (bind _returnvalue_19 (`OSCManager.ConvertStringToOSCAddress` "/unreal/camera/fstops/max")) ; Change the Apeature Size
  (`OSCServer.BindEventToOnOSCAddressPatternMatchesPath` _output_get _returnvalue_19 (delegate `Set Camera F Stops Max`))
  (bind _returnvalue_20 (`OSCManager.ConvertStringToOSCAddress` "/unreal/camera/fstops/min")) ; Changing the Max Apature / F Stops Min
  (`OSCServer.BindEventToOnOSCAddressPatternMatchesPath` _output_get _returnvalue_20 (delegate `Set Camera F Stops Min`))
  (bind _returnvalue_21 (`OSCManager.ConvertStringToOSCAddress` "/unreal/camera/blades")) ; Changing some virtual camera paramters\nI don't think this works
  (`OSCServer.BindEventToOnOSCAddressPatternMatchesPath` _output_get _returnvalue_21 (delegate `Set Camera Diaphram Blades`))
  (bind _returnvalue_22 (`OSCManager.ConvertStringToOSCAddress` "/unreal/ndisplay/level")) ; This is what does the level loading on the \nstreamdeck with bitfocus companion
  (`OSCServer.BindEventToOnOSCAddressPatternMatchesPath` _output_get _returnvalue_22 (delegate `Change Current Level`)))

(event `Set Camera DOF Blur Radius`
  (params (AddressPattern :type "OSCAddress Structure (by ref)") (Message :type "OSCMessage Structure (by ref)") (IPAddress :type String) (Port :type Integer))
  (bind _value (`OSCManager.GetFloat` Message))
  (set `CameraComponent.PostProcessSettings` (make `PostProcessSettings` :`DepthOfFieldDepthBlurRadius` (`KismetMathLibrary.FClamp` _value 0.0 4.0)) (`CineCameraActor.GetCineCameraComponent` (`/nDisplay/Blueprints/ReprojectionCamera/BP_IncameraSettings.ReprojectedCineCamera` (`self.Incamera`)))))

(event `Reset OSC Ping Seconds`
  (params (AddressPattern :type "OSCAddress Structure (by ref)") (Message :type "OSCMessage Structure (by ref)") (IPAddress :type String) (Port :type Integer))
  (set `self.Last OSC Message` 0) ; This is just resetting a seconds since last\nmessage, used to tell if the OSC server has\nstopped working.
)

(event `Change FOV Offset`
  (params (AddressPattern :type "OSCAddress Structure (by ref)") (Message :type "OSCMessage Structure (by ref)") (IPAddress :type String) (Port :type Integer))
  (bind _value (`OSCManager.GetFloat` Message))
  (`self.Nudge FOV Offset` (> _value 0.0)) ; Increment the FOV Offset
  (set `self.Last OSC Message` 0))

(event `Set Camera F Stops Max`
  (params (AddressPattern :type "OSCAddress Structure (by ref)") (Message :type "OSCMessage Structure (by ref)") (IPAddress :type String) (Port :type Integer))
  (bind _value (`OSCManager.GetFloat` Message))
  (set `CameraComponent.PostProcessSettings` (make `PostProcessSettings` :`DepthOfFieldFstop` (`KismetMathLibrary.FClamp` _value 1.2 32.0)) (`CineCameraActor.GetCineCameraComponent` (`/nDisplay/Blueprints/ReprojectionCamera/BP_IncameraSettings.ReprojectedCineCamera` (`self.Incamera`)))))

(event `Set Camera Diaphram Blades`
  (params (AddressPattern :type "OSCAddress Structure (by ref)") (Message :type "OSCMessage Structure (by ref)") (IPAddress :type String) (Port :type Integer))
  (bind _value (`OSCManager.GetFloat` Message))
  (set `CameraComponent.PostProcessSettings` (make `PostProcessSettings` :`DepthOfFieldBladeCount` (`KismetMathLibrary.FTrunc` (`KismetMathLibrary.FClamp` _value 4.0 16.0))) (`CineCameraActor.GetCineCameraComponent` (`/nDisplay/Blueprints/ReprojectionCamera/BP_IncameraSettings.ReprojectedCineCamera` (`self.Incamera`)))))

(event `Update Stage Location YZ`
  (params (AddressPattern :type "OSCAddress Structure (by ref)") (Message :type "OSCMessage Structure (by ref)") (IPAddress :type String) (Port :type Integer))
  (bind _value (`OSCManager.GetFloat` Message)) ; The first axis comes in on index 0
  (set `self.Stage Location Y` _value)
  (bind _value_2 (`OSCManager.GetFloat` Message 1)) ; The second axis comes in on index 1
  (set `self.Stage Location Z` _value_2)
  (set `self.Last OSC Message` 0))

(event `Update Stage Rotation YZ`
  (params (AddressPattern :type "OSCAddress Structure (by ref)") (Message :type "OSCMessage Structure (by ref)") (IPAddress :type String) (Port :type Integer))
  (bind _value (`OSCManager.GetFloat` Message))
  (set `self.Stage Rotation Z` _value)
  (bind _value_2 (`OSCManager.GetFloat` Message 1))
  (set `self.Stage Rotation Y` _value_2)
  (set `self.Last OSC Message` 0))

(event `Enable Chromakey Blur`
  (params (AddressPattern :type "OSCAddress Structure (by ref)") (Message :type "OSCMessage Structure (by ref)") (IPAddress :type String) (Port :type Integer))
  (`/nDisplay/Blueprints/ReprojectionCamera/BP_IncameraSettings.ApplyChromakeyBlur` (`self.Incamera`))
  (set `self.Last OSC Message` 0))

(event `Nudge Stage RotX`
  (params (AddressPattern :type "OSCAddress Structure (by ref)") (Message :type "OSCMessage Structure (by ref)") (IPAddress :type String) (Port :type Integer))
  (bind _value (`OSCManager.GetInt32` Message))
  (`self.Nudge Projection Rotation X` _value))

(event `Adjust Frustum Feather`
  (params (AddressPattern :type "OSCAddress Structure (by ref)") (Message :type "OSCMessage Structure (by ref)") (IPAddress :type String) (Port :type Integer))
  (bind _value (`OSCManager.GetFloat` Message))
  (set `/nDisplay/Blueprints/ReprojectionCamera/BP_IncameraSettings.InnerCameraSoftEdge` (`KismetMathLibrary.Conv_DoubleToVector` _value) (`self.Incamera`)) ; This only seems to set it temporarlly?
)

(event `Set Camera DOF Focal Distance`
  (params (AddressPattern :type "OSCAddress Structure (by ref)") (Message :type "OSCMessage Structure (by ref)") (IPAddress :type String) (Port :type Integer))
  (bind _value (`OSCManager.GetFloat` Message))
  (set `CameraComponent.PostProcessSettings` (make `PostProcessSettings` :`DepthOfFieldFocalDistance` (`KismetMathLibrary.FClamp` _value 1.0 1000.0)) (`CineCameraActor.GetCineCameraComponent` (`/nDisplay/Blueprints/ReprojectionCamera/BP_IncameraSettings.ReprojectedCineCamera` (`self.Incamera`)))))

(event `Set Camera F Stops Min`
  (params (AddressPattern :type "OSCAddress Structure (by ref)") (Message :type "OSCMessage Structure (by ref)") (IPAddress :type String) (Port :type Integer))
  (bind _value (`OSCManager.GetFloat` Message))
  (set `CameraComponent.PostProcessSettings` (make `PostProcessSettings` :`DepthOfFieldMinFstop` (`KismetMathLibrary.FClamp` _value 1.2 32.0)) (`CineCameraActor.GetCineCameraComponent` (`/nDisplay/Blueprints/ReprojectionCamera/BP_IncameraSettings.ReprojectedCineCamera` (`self.Incamera`)))))

(event `Change Current Level`
  (params (AddressPattern :type "OSCAddress Structure (by ref)") (Message :type "OSCMessage Structure (by ref)") (IPAddress :type String) (Port :type Integer))
  (bind _value (`OSCManager.GetString` Message))
  (bind _boutsuccess (`LevelStreamingDynamic.LoadLevelInstance` _value)) ; This is an instance load of a specified level
  (if _boutsuccess
    (`KismetSystemLibrary.PrintString` "Loaded Level")
    (`GameplayStatics.UnloadStreamLevel` (`KismetStringLibrary.Conv_StringToName` (`self.PreviousLevel`))) ; This unloads the previous level
    (`KismetSystemLibrary.PrintString` "Un-Loaded Level")
    (set `self.PreviousLevel` _value) ; Set the previous level as the \ncurrent level for next time we call this
    (else
      (`KismetSystemLibrary.PrintString` "Error Loading Level"))))

(event `Update Location X`
  (params (AddressPattern :type "OSCAddress Structure (by ref)") (Message :type "OSCMessage Structure (by ref)") (IPAddress :type String) (Port :type Integer))
  (bind _value (`OSCManager.GetFloat` Message))
  (set `self.Stage Location X` _value)
  (set `self.Last OSC Message` 0))

(event `Update Stage Rotation X`
  (params (AddressPattern :type "OSCAddress Structure (by ref)") (Message :type "OSCMessage Structure (by ref)") (IPAddress :type String) (Port :type Integer))
  (bind _value (`OSCManager.GetFloat` Message))
  (set `self.Stage Rotation X` _value)
  (set `self.Last OSC Message` 0))

(event `Nudge Stage RotZ`
  (params (AddressPattern :type "OSCAddress Structure (by ref)") (Message :type "OSCMessage Structure (by ref)") (IPAddress :type String) (Port :type Integer))
  (bind _value (`OSCManager.GetInt32` Message)) ; Using an INT because we're coming from \nBitfocus companion for this and it can send\nintegers...unlike touchOSC
  (`self.Nudge Projection Rotation Z` _value))

(event `Nudge Stage RotY`
  (params (AddressPattern :type "OSCAddress Structure (by ref)") (Message :type "OSCMessage Structure (by ref)") (IPAddress :type String) (Port :type Integer))
  (bind _value (`OSCManager.GetInt32` Message))
  (`self.Nudge Projection Rotation Y` _value))

(event `Message Toggle`
  (params (AddressPattern :type "OSCAddress Structure (by ref)") (Message :type "OSCMessage Structure (by ref)") (IPAddress :type String) (Port :type Integer))
  (bind _value (`OSCManager.GetInt32` Message)) ; Other OSC sources might be integers
  (if (`KismetMathLibrary.Conv_IntToBool` _value)
    (`KismetSystemLibrary.ExecuteConsoleCommand` "EnableAllScreenMessages" null) ; Disable all screen messages
    (`KismetSystemLibrary.PrintString` "Messages Enabled")
    (set `self.Last OSC Message` 0)
    (else
      (`KismetSystemLibrary.PrintString` "Messages Disabled")
      (`KismetSystemLibrary.ExecuteConsoleCommand` "DisableAllScreenMessages" null) ; Turn off screen messages with a \nconsole command
      (set `self.Last OSC Message` 0))))

(event `Enable Chromakey Capture`
  (params (AddressPattern :type "OSCAddress Structure (by ref)") (Message :type "OSCMessage Structure (by ref)") (IPAddress :type String) (Port :type Integer))
  (`/nDisplay/Blueprints/ReprojectionCamera/BP_IncameraSettings.CaptureChromakey` (`self.Incamera`))
  (set `self.Last OSC Message` 0))

(event `StartOnlineSesh`
  (params (AddressPattern :type "OSCAddress Structure (by ref)") (Message :type "OSCMessage Structure (by ref)") (IPAddress :type String) (Port :type Integer))
  (bind _value (`OSCManager.GetFloat` Message))
  (if (> _value 0.0)
    (bind _returnvalue (`MultiUserClientStatics.StartMultiUserDefaultConnection`))
    (if _returnvalue
      (`KismetSystemLibrary.PrintString` "Joined multi-user sesh")
      (else
        (`KismetSystemLibrary.PrintString` "Failed to join multi user sesh")))))

(event `Test ACCXYZ`
  (params (AddressPattern :type "OSCAddress Structure (by ref)") (Message :type "OSCMessage Structure (by ref)") (IPAddress :type String) (Port :type Integer)))

(event `Key|J`
  (params (Key :type "Key Structure"))
  ;[1 1 1] This function is for multi-playet function (to replicate data between clients using the multiplayer game mode) - it's just an idea! probably not the best way to achieve this
  (:`Pressed`
    (`KismetArrayLibrary.Array_Clear` (`self.OnlineSessions`))
    (bind _results (`FindSessionsCallbackProxy.FindSessions` null)
      (:`then`
        (bind _output_get (set `self.OnlineSessions` _results))
        (for _array_element _output_get
          (if (!= (`FindSessionsCallbackProxy.GetCurrentPlayers` _array_element) (`FindSessionsCallbackProxy.GetMaxPlayers` _array_element))
            (set `self.SessionFound?` true)
            (set `self.AvailableSession` _array_element)
            (break)))
        (if (`self.SessionFound?`)
          (`KismetSystemLibrary.PrintString` "Found online session - Joining...." true true (struct :`G` 0.66 :`B` 1.0 :`A` 1.0) 4.0)
          (`JoinSessionCallbackProxy.JoinSession` (`GameplayStatics.GetPlayerController` 0) (`self.AvailableSession`)))))))

(event `Check OSC Server`
  ;[1 1 1] Restart the OSC server after more than 30 seconds of no new messages
  (if (not (`OSCServer.IsActive` (`self.OSC Server`)))
    (`KismetSystemLibrary.PrintString` "Restarting OSC Server")
    (`self.StartOSC`)))

(event `Nudge Projection Rotation Z`
  (params (`Z Rotation Nudge Direction` :type Integer))
  (bind _root_offset (`/Game/WarpMesh/BP_WarpMonitor.root Offset` (`self.Mesh Wall`)))
  (bind (_relativerotation_roll _relativerotation_pitch _relativerotation_yaw) (`KismetMathLibrary.BreakRotator` (`SceneComponent.RelativeRotation` _root_offset)))
  (bind (_relativerotation_roll_2 _relativerotation_pitch_2 _relativerotation_yaw_2) (`KismetMathLibrary.BreakRotator` (`SceneComponent.RelativeRotation` _root_offset)))
  ;[1 1 1] Root correction for projection Z rotation
  (if (> `Z Rotation Nudge Direction` 0)
    (`SceneComponent.K2_SetRelativeRotation` _root_offset (`KismetMathLibrary.MakeRotator` 0.0 0.0 (+ _relativerotation_yaw 0.5)) false false)
    (else
      (`SceneComponent.K2_SetRelativeRotation` _root_offset (`KismetMathLibrary.MakeRotator` 0.0 0.0 (+ _relativerotation_yaw_2 -0.5)) false false))))

(event `Nudge Projection Rotation Y`
  (params (`Y Rotation Nudge DIrection` :type Integer))
  (bind _root_offset (`/Game/WarpMesh/BP_WarpMonitor.root Offset` (`self.Mesh Wall`)))
  (bind (_relativerotation_roll _relativerotation_pitch) (`KismetMathLibrary.BreakRotator` (`SceneComponent.RelativeRotation` _root_offset)))
  (bind (_relativerotation_roll_2 _relativerotation_pitch_2) (`KismetMathLibrary.BreakRotator` (`SceneComponent.RelativeRotation` _root_offset)))
  ;[1 1 1] Root correction for projection Y rotation
  (if (> `Y Rotation Nudge DIrection` 0)
    (`SceneComponent.K2_SetRelativeRotation` _root_offset (`KismetMathLibrary.MakeRotator` 0.0 (+ _relativerotation_pitch 0.5)) false false)
    (else
      (`SceneComponent.K2_SetRelativeRotation` _root_offset (`KismetMathLibrary.MakeRotator` 0.0 (+ _relativerotation_pitch_2 -0.5)) false false))))

(event `Nudge Projection Rotation X`
  (params (`X Rotation Nudge Direction` :type Integer))
  (bind _root_offset (`/Game/WarpMesh/BP_WarpMonitor.root Offset` (`self.Mesh Wall`)))
  (bind _relativerotation_roll (`KismetMathLibrary.BreakRotator` (`SceneComponent.RelativeRotation` _root_offset)))
  (bind _relativerotation_roll_2 (`KismetMathLibrary.BreakRotator` (`SceneComponent.RelativeRotation` _root_offset)))
  ;[1 1 1] Root correction for projection X rotation
  (if (> `X Rotation Nudge Direction` 0)
    (`SceneComponent.K2_SetRelativeRotation` _root_offset (`KismetMathLibrary.MakeRotator` (+ _relativerotation_roll_2 0.5)) false false)
    (else
      (`SceneComponent.K2_SetRelativeRotation` _root_offset (`KismetMathLibrary.MakeRotator` (+ _relativerotation_roll -0.5)) false false))))

(fn `Nudge FOV Offset`
  (params (Direction :type Boolean))
  (bind _incamera (`self.Incamera`))
  (bind _fovmultiplier (`/nDisplay/Blueprints/ReprojectionCamera/BP_IncameraSettings.FOVMultiplier` _incamera))
  (bind _returnvalue (`KismetMathLibrary.FClamp` (+ _fovmultiplier 0.1) 0.1 3.0))
  ;[1 1 1] FOV Offset
  (if Direction
    (set `/nDisplay/Blueprints/ReprojectionCamera/BP_IncameraSettings.FOVMultiplier` _returnvalue _incamera)
    (`KismetSystemLibrary.PrintString` (`KismetStringLibrary.Concat_StrStr` "Nudged FOV: " (`KismetStringLibrary.Conv_DoubleToString` _returnvalue)))
    (else
      (set `/nDisplay/Blueprints/ReprojectionCamera/BP_IncameraSettings.FOVMultiplier` (`KismetMathLibrary.FClamp` (+ _fovmultiplier -0.1) 0.1 3.0) _incamera))))

(fn `Stage Track`
  (`SceneComponent.K2_SetRelativeLocationAndRotation` (`self.DisplayClusterRootComponent`) (`KismetMathLibrary.MakeVector` (`self.Stage Location X`) (`self.Stage Location Y`) (`self.Stage Location Z`)) (`KismetMathLibrary.MakeRotator` (`self.Stage Rotation X`) (`self.Stage Rotation Y`) (`self.Stage Rotation Z`)) false false))

(fn `UserConstructionScript`)