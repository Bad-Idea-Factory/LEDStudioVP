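; Virtual production actor that moves a referenced Camera in the editor from tracking data received over OSC.
; EditorTick recreates the OSC server if inactive, then applies stored location and rotation as the camera's relative transform.
; Handlers bound to the location and rotation addresses fill those values from message floats.
; As wired, only location X updates, and rotation Y and Z both read index 1.
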(event `self.EditorTick`
  (params (DeltaSeconds :type "Float (single-precision)"))
  (`self.Check OSC Server`)
  (`self.Track Cam In Editor`))

(event `Track Cam In Editor`
  (bind _camera (`self.Camera`))
  (`self.K2_SetActorRelativeLocation` _camera (`KismetMathLibrary.MakeVector` (`self.Location X`) (`self.Location Y`) (`self.Location Z`)) false false)
  (`self.K2_SetActorRelativeRotation` _camera (`KismetMathLibrary.MakeRotator` (`self.Rotation X`) (`self.Rotation Y`) (`self.Rotation Z`)) false false))

(event `Check OSC Server`
  ;[1 1 1] Restart the OSC server after more than 30 seconds of no new messages
  (if (not (`OSCServer.IsActive` (`self.OSC Server`)))
    (`KismetSystemLibrary.PrintString` "Restarting OSC Server")
    (`self.OSC VRPN Translator`)))

(event `OSC VRPN Translator`
  ;[1 1 1] Get the OSC Messages and set the location and rotation parameters
  (bind _returnvalue (`OSCManager.CreateOSCServer` (`self.OSC IP Address`) (`self.OSC Port`) false true))
  (bind _output_get (set `self.OSC Server` _returnvalue))
  (bind _returnvalue_2 (`OSCManager.ConvertStringToOSCAddress` "/unrealvp/tracksend/location"))
  (`OSCServer.BindEventToOnOSCAddressPatternMatchesPath` _output_get _returnvalue_2 (delegate `Get VRPN Location From OSC`))
  (bind _returnvalue_3 (`OSCManager.ConvertStringToOSCAddress` "/unrealvp/tracksend/rotation"))
  (`OSCServer.BindEventToOnOSCAddressPatternMatchesPath` _output_get _returnvalue_3 (delegate `Get VRPN Rotation from OSC`)))

(event `Get VRPN Location From OSC`
  (params (AddressPattern :type "OSCAddress Structure (by ref)") (Message :type "OSCMessage Structure (by ref)") (IPAddress :type String) (Port :type Integer))
  ;[1 1 1] Get the OSC Messages and set the location and rotation parameters
  (bind _value (`OSCManager.GetFloat` Message))
  (set `self.Location X` _value))

(event `Get VRPN Rotation from OSC`
  (params (AddressPattern :type "OSCAddress Structure (by ref)") (Message :type "OSCMessage Structure (by ref)") (IPAddress :type String) (Port :type Integer))
  ;[1 1 1] Get the OSC Messages and set the location and rotation parameters
  (bind _value (`OSCManager.GetFloat` Message))
  (set `self.Rotation X` _value)
  (bind _value_2 (`OSCManager.GetFloat` Message 1))
  (set `self.Rotation Y` _value_2)
  (bind _value_3 (`OSCManager.GetFloat` Message 1))
  (set `self.Rotation Z` _value_3))

(fn `UserConstructionScript`)